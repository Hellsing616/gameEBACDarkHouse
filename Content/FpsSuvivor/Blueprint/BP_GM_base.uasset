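; Base game mode for a zombie wave survival level, showing HUD start, wave and win messages.
; After timed intro delays, CreateWave spawns BP_ZumbieGirl at three points, each receiving the current wave number in zombies.
; TotalEnemy equals only one point's count; DecEnemies lowers it and calls WavesIncrements.
; At zero or below, WavesIncrements starts the next wave or, after the last, shows victory and opens LeviatanMap.
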(event Custom|GameStart
  ;[1 1 1] Spawn dos Zumbies
  (CallFunction|CreateWave))

(event Custom|WavesIncrements
  ;[1 1 1] Incremento a onde inimigos
  (if (<= (Variables|Default|GetTotalEnemy) 0)
    (bind _output_get (Variables|Default|SetCurrentWaves (+ (Variables|Default|GetCurrentWaves) 1)))
    (if (> _output_get (Variables|Default|GetTotalWaves))
      ;[1 1 1] ganhou a fase
      (Default|ShowWinGame (Variables|/Game/FpsSuvivor/Blueprint/BP_FirstPersonCharacter.BP_FirstPersonCharacter_C|GetHUD (stale _asbp_first_person_character)))
      (Utilities|FlowControl|Delay 5.0)
      (Game|OpenLevel(byName) "LeviatanMap")
      (else
        (bind _asbp_first_person_character (Utilities|Casting|CastToBP_FirstPersonCharacter (Game|GetPlayerCharacter 0)))
        (Default|ShowMessagemWave (Variables|/Game/FpsSuvivor/Blueprint/BP_FirstPersonCharacter.BP_FirstPersonCharacter_C|GetHUD _asbp_first_person_character))
        (Utilities|FlowControl|Delay 5.0)
        (CallFunction|CreateWave)))))

(event EventBeginPlay
  ;[1 1 1] Start Game
  (Variables|Default|SetTotalWaves 2)
  (Variables|Default|SetCurrentWaves 1)
  (Utilities|FlowControl|Delay 3.0)
  (bind _asbp_first_person_character (Utilities|Casting|CastToBP_FirstPersonCharacter (Game|GetPlayerCharacter 0)))
  (Default|ShowStartLevelMessage (Variables|/Game/FpsSuvivor/Blueprint/BP_FirstPersonCharacter.BP_FirstPersonCharacter_C|GetHUD _asbp_first_person_character))
  (Utilities|FlowControl|Delay 2.0)
  (Default|ShowMessagemWave (Variables|/Game/FpsSuvivor/Blueprint/BP_FirstPersonCharacter.BP_FirstPersonCharacter_C|GetHUD _asbp_first_person_character))
  (Utilities|FlowControl|Delay 3.0)
  (CallFunction|GameStart))

(event EventTick
  (params (DeltaSeconds :type Float%20%28single-precision%29)))

(fn ConstructionScript)

(fn CreateWave
  (bind _output_get (Variables|Default|SetTotalEnemy (* (Variables|Default|GetCurrentWaves) 1)))
  (bind _output_get_2 (Variables|Default|SetEnemysPerPoint (/ _output_get 1)))
  (Utilities|FlowControl|ForLoopwithBreak 1 _output_get_2
    (:LoopBody
      (Game|SpawnActorfromClass "/Game/FpsSuvivor/Blueprint/BP_ZumbieGirl.BP_ZumbieGirl_C" (Variables|Default|GetSpawnPoint1) "Undefined" "MultiplyWithRoot" 0 0))
    (:Completed
      (Utilities|FlowControl|ForLoopwithBreak 1 _output_get_2
        (:LoopBody
          (Game|SpawnActorfromClass "/Game/FpsSuvivor/Blueprint/BP_ZumbieGirl.BP_ZumbieGirl_C" (Variables|Default|GetSpawnPoint2) "Undefined" "MultiplyWithRoot" 0 0))
        (:Completed
          (Utilities|FlowControl|ForLoopwithBreak 1 _output_get_2
            (:LoopBody
              (Game|SpawnActorfromClass "/Game/FpsSuvivor/Blueprint/BP_ZumbieGirl.BP_ZumbieGirl_C" (Variables|Default|GetSpawnPoint3) "Undefined" "MultiplyWithRoot" 0 0))))))))

(fn DecEnemies
  (Variables|Default|SetTotalEnemy (- (Variables|Default|GetTotalEnemy) 1))
  (CallFunction|WavesIncrements))