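; BP_ZumbieGirl is a zombie enemy that chases and attacks the player, with random speed raised on sighting via PawnSensing.
; AIMoveTo toward player controller 0 alternates with an attack montage, whose notify triggers a sphere overlap that damages BP_FirstPersonCharacter.
; Point damage reduces health and plays a hit reaction or triggers death.
; Death stops movement, plays a montage, then after delays decrements BP_GM_base's enemy count and destroys the actor.
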(event OnSeePawn(PawnSensing)
  (params (Pawn :type Pawn%20Object%20Reference))
  ;[1 1 1] Muda a velocidade do inimigo quando estiver perto do player
  (Variables|/Script/Engine.CharacterMovementComponent|SetMaxWalkSpeed (Variables|Character|GetCharacterMovement) (Math|Random|RandomFloatinRange 3e+02 6e+02)))

(event Custom|EventCustom
  ;[1 1 1] mover inimigo automaticamento
  (if (not (Variables|Default|GetisDeath?))
    (AI|AIMoveTo self "0, 0, 0" (Game|GetPlayerController 0) 6e+01 false
      (:OnSuccess
        (CallFunction|AttacPlayer))
      (:OnFail
        (CallFunction|EventCustom)))))

(event Custom|AttacPlayer
  ;[1 1 1] atacar player
  (if (not (Variables|Default|GetisDeath?))
    (Animation|Montage|PlayMontage (Variables|Character|GetMesh) "/Game/FpsSuvivor/Character/inimigos/ZombieGirl/Animation/zombie_attack_Montage.zombie_attack_Montage"
      (:OnCompleted
        (CallFunction|EventCustom))
      (:OnNotifyBegin
        (bind (_outactors _returnvalue) (Collision|SphereOverlapActors (Transformation|GetWorldLocation (Variables|Default|GetArrowAttack)) 1e+02 (Utilities|Array|MakeArray "ObjectTypeQuery3") "/Game/FpsSuvivor/Blueprint/BP_FirstPersonCharacter.BP_FirstPersonCharacter_C" (Utilities|Array|MakeArray self)))
        (if _returnvalue
          (for _array_element _outactors
            (Game|Damage|ApplyDamage _array_element 2e+01 (Pawn|GetController) self "/Script/Engine.DamageType")))))))

(event Custom|Death
  (bind _charactermovement (Variables|Character|GetCharacterMovement))
  ;[1 1 1] Death
  (Variables|Default|SetisDeath? true)
  (Class|NavMovementComponent|StopActiveMovement _charactermovement)
  (Components|Movement|StopMovementImmediately _charactermovement)
  (Animation|PlayAnimMontage self "/Game/FpsSuvivor/Character/inimigos/ZombieGirl/Animation/zombie_death_Montage.zombie_death_Montage" 1.0 "None")
  (bind _asbp_gm_base (Utilities|Casting|CastToBP_GM_base (Game|GetGameMode)))
  (Utilities|FlowControl|Delay 2e+01)
  (Default|DecEnemies _asbp_gm_base)
  (Utilities|FlowControl|Delay 5.0)
  (Actor|DestroyActor))

(event EventBeginPlay
  ;[1 1 1] Velocidade ao iniciar o jogo
  (Variables|/Script/Engine.CharacterMovementComponent|SetMaxWalkSpeed (Variables|Character|GetCharacterMovement) (Math|Random|RandomFloatinRange 1e+02 3e+02))
  (CallFunction|EventCustom))

(event Collision|EventActorBeginOverlap
  (params (OtherActor :type Actor%20Object%20Reference)))

(event Game|Damage|EventPointDamage
  (params (Damage :type Float%20%28single-precision%29) (DamageType :type Damage%20Type%20Object%20Reference) (HitLocation :type Vector :default "0, 0, 0") (HitNormal :type Vector :default "0, 0, 0") (HitComponent :type Primitive%20Component%20Object%20Reference) (BoneName :type Name :default "None") (ShotFromDirection :type Vector :default "0, 0, 0") (InstigatedBy :type Controller%20Object%20Reference) (DamageCauser :type Actor%20Object%20Reference) (HitInfo :type Hit%20Result%20Structure%20%28by%20ref%29))
  ;[1 1 1] Dano no inimigo
  (if (not (Variables|Default|GetisDeath?))
    (bind _output_get (Variables|Default|SetHealth (- (Variables|Default|GetHealth) Damage)))
    (if (<= _output_get 0.0)
      (CallFunction|Death)
      (else
        (Animation|Montage|PlayMontage (Variables|Character|GetMesh) "/Game/FpsSuvivor/Character/inimigos/ZombieGirl/Animation/Zombie_Reaction_Hit_mixamo_com_Montage.Zombie_Reaction_Hit_mixamo_com_Montage")))))

(fn ConstructionScript)